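; BP_NormalRifle is a rifle weapon that fires bullets from a limited magazine and reloads from a count of spare magazines.
; The attack event, while rounds remain, uses one and spawns a BP_Bullet at the AimPoint transform of its parent actor.
; The reload event, while spare magazines remain, consumes one and refills the current magazine to its maximum, discarding any leftover rounds.
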(event EventWeaponReload
  (if (> (Variables|Default|GetNumberOfMagazine) 0.0)
    (Variables|Default|SetNumberOfMagazine (- (Variables|Default|GetNumberOfMagazine) 1.0))
    (Variables|Default|SetMagazine (Variables|Default|GetMaxMagazine))))

(event EventWeaponAttack
  (if (> (Variables|Default|GetMagazine) 0)
    (Variables|Default|SetMagazine (- (Variables|Default|GetMagazine) 1))
    (Game|SpawnActorfromClass "/Game/Actors/Weapons/BP_Bullet.BP_Bullet_C" (Transformation|GetWorldTransform (Variables|/Game/Actors/BP_CharacterBase.BP_CharacterBase_C|GetAimPoint (Variables|Default|GetParentActor))) "Undefined" "MultiplyWithRoot" 0 0)))

(fn ConstructionScript)