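; BP_WeaponManager is a weapon manager that gets its parent actor as a Character and routes combat actions to the selected weapon.
; On BeginPlay it caches that Character and builds an array of beam rifle, normal rifle and beam saber.
; SwapWeapon cycles the active index with modulo wraparound.
; Attack and Reload forward message calls to the weapon at that index.
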(event Custom|SwapWeapon
  ;[0.15 0.15 0.15 0.5] 무기를 지정할 번호 1증가. 해당 번호로 배열에 접근.
  (Variables|Default|SetNowWeapon (Math|Integer|%(Integer) (+ (Variables|Default|GetNowWeapon) 1) (Variables|Default|GetWeaponsCount))))

(event Custom|Attack
  (Class|WeaponAction|WeaponAttack(Message) (Utilities|Array|Get(acopy) (Variables|Default|GetWeapons) (Variables|Default|GetNowWeapon))))

(event Custom|Reload
  (Class|WeaponAction|WeaponReload(Message) (Utilities|Array|Get(acopy) (Variables|Default|GetWeapons) (Variables|Default|GetNowWeapon))))

(event EventBeginPlay
  (bind _as캐릭터 (Utilities|Casting|CastToCharacter (Actor|GetParentActor)))
  (Variables|Default|SetParentCharacter _as캐릭터)
  (Variables|Default|SetWeapons (Utilities|Array|MakeArray (Variables|Default|GetWeaponBeamRifle) (Variables|Default|GetWeaponNormalRifle) (Variables|Default|GetWeaponBeamSaber))))

(fn ConstructionScript)