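; Beam rifle weapon Blueprint that handles an energy-gated attack from its parent actor's aim point.
; WeaponAttack checks for remaining energy, sets it to UseEnergyAmount minus itself (zero), runs Shooting, then passes the rifle's damage to the parent actor.
; Shooting line-traces on Visibility toward the aim's forward vector times range, without adding the start location, and leaves the hit unused.
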(event EventWeaponAttack
  (if (> (Variables|Default|GetLeftEnergyAmount) 0)
    (Variables|Default|SetLeftEnergyAmount (- (Variables|Default|GetUseEnergyAmount) (Variables|Default|GetUseEnergyAmount)))
    (Utilities|Shooting)
    (Class|BIActorGetAttack|GetDamage(Message) (Variables|Default|GetParentActor) (Variables|Default|GetBeamRifleDamage))))

(fn ConstructionScript)