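; BP_Enemy is an enemy pawn that can detect, approach and take damage from interactions in the game.
; SeePlayer and Attackable run sphere overlaps around it, using sight radius and attack range, to return the first BP_Player found.
; MovetoPlayer adds movement input toward a given location, and GetDamage subtracts from Health with no death handling.
; The file contains no tick or decision logic, so these act as building blocks called from outside.
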(event EventGetDamage
  (params (Damage :type Float%20%28double-precision%29))
  (Variables|Default|SetHealth (- (Variables|Default|GetHealth) Damage)))

(event EventMovetoPlayer
  (params (LocationToGo :type Vector :default "0, 0, 0"))
  (Pawn|Input|AddMovementInput (- LocationToGo (Transformation|GetActorLocation)) 1.0 false))

(fn ConstructionScript)

(fn Attackable
  (bind (_outactors _returnvalue) (Collision|SphereOverlapActors (Transformation|GetActorLocation) (Variables|Default|GetAttackRange) (Utilities|Array|MakeArray "ObjectTypeQuery3") "/Game/Actors/Player/BP_Player.BP_Player_C"))
  (if _returnvalue
    (return (Utilities|Array|Get(acopy) _outactors))
    (else
      (return 0))))

(fn SeePlayer
  (bind (_outactors _returnvalue) (Collision|SphereOverlapActors (Transformation|GetActorLocation) (Variables|Default|GetSightRadius) (Utilities|Array|MakeArray "ObjectTypeQuery3") "/Game/Actors/Player/BP_Player.BP_Player_C"))
  (if _returnvalue
    (return (Utilities|Array|Get(acopy) _outactors))
    (else
      (return 0))))