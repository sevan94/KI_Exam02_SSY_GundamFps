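; BP_Enemy is an enemy character Blueprint that provides proximity checks for detecting the player.
; Attackable and SeePlayer each run a sphere overlap at the enemy's location, filtered to BP_Player pawns, using AttackRange and SightRadius respectively.
; Each returns the first overlapped player, or nothing on a miss; sight is purely radius-based, with no line-of-sight or facing test.
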(fn ConstructionScript)

(fn Attackable
  (bind (_outactors _returnvalue) (Collision|SphereOverlapActors (Transformation|GetActorLocation) (Variables|Default|GetAttackRange) (Utilities|Array|MakeArray "ObjectTypeQuery3") "/Game/Character/TempCharacters/Player/BP_Player.BP_Player_C"))
  (if _returnvalue
    (return (Utilities|Array|Get(acopy) _outactors))
    (else
      (return 0))))

(fn SeePlayer
  (bind (_outactors _returnvalue) (Collision|SphereOverlapActors (Transformation|GetActorLocation) (Variables|Default|GetSightRadius) (Utilities|Array|MakeArray "ObjectTypeQuery3") "/Game/Character/TempCharacters/Player/BP_Player.BP_Player_C"))
  (if _returnvalue
    (return (Utilities|Array|Get(acopy) _outactors))
    (else
      (return 0))))