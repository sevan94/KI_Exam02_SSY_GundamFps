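; BP_Player is a flying player character with planar and vertical movement and a limited speed boost.
; Enhanced Input actions feed AddMovementInput along world axes, and IA_Boost switches MaxFlySpeed between normal and boost speeds.
; While boosting, Tick drains LeftBoostAmount, prints it for debugging, and ends the boost once the IsBoostLeft check fails.
; No boost refill happens here.
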(event Custom|BoostDeactive
  ;[0.15 0.15 0.15 0.5] 부스트 비활성화
  (Variables|/Script/Engine.CharacterMovementComponent|SetMaxFlySpeed (Variables|Character|GetCharacterMovement) (Variables|Default|GetNormalSpeed))
  (Variables|Default|SetbIsBoosting false))

(event Custom|BoostActive
  ;[0.15 0.15 0.15 0.5] 부스트 활성화
  (Utilities|IsBoostLeft
    (:True
      (Variables|/Script/Engine.CharacterMovementComponent|SetMaxFlySpeed (Variables|Character|GetCharacterMovement) (Variables|Default|GetBoostSpeed))
      (Variables|Default|SetbIsBoosting true))))

(event Input|EnhancedActionEvents|EnhancedInputActionIA_PlanarMotion
  (params (ActionValue :type Vector%202D%20Structure) (ElapsedSeconds :type Float%20%28double-precision%29) (TriggeredSeconds :type Float%20%28double-precision%29) (InputAction :type Input%20Action%20Object%20Reference :default "/Game/Input/IA_PlanarMotion.IA_PlanarMotion"))
  ;[0.15 0.15 0.15 0.5] 평면(앞뒤좌우)이동
  (bind _output_get (Variables|Default|SetDirection (Math|Vector|MakeVector (.x ActionValue) (.y ActionValue) 0.0)))
  (Pawn|Input|AddMovementInput _output_get 1.0 false))

(event Input|EnhancedActionEvents|EnhancedInputActionIA_Up
  (params (ActionValue :type Boolean) (ElapsedSeconds :type Float%20%28double-precision%29) (TriggeredSeconds :type Float%20%28double-precision%29) (InputAction :type Input%20Action%20Object%20Reference :default "/Game/Input/IA_Up.IA_Up"))
  ;[0.15 0.15 0.15 0.5] 위로 올라가는 동작
  (if ActionValue
    (bind _output_get (Variables|Default|SetDirection (Math|Vector|MakeVector 0.0 0.0 (Variables|Default|GetTrueAsNumber))))
    (Pawn|Input|AddMovementInput _output_get 1.0 false)))

(event Input|EnhancedActionEvents|EnhancedInputActionIA_Down
  (params (ActionValue :type Boolean) (ElapsedSeconds :type Float%20%28double-precision%29) (TriggeredSeconds :type Float%20%28double-precision%29) (InputAction :type Input%20Action%20Object%20Reference :default "/Game/Input/IA_Down.IA_Down"))
  ;[0.15 0.15 0.15 0.5] 아래로 내려가는 동작
  (if ActionValue
    (bind _output_get (Variables|Default|SetDirection (Math|Vector|MakeVector 0.0 0.0 (* (Variables|Default|GetTrueAsNumber) (Variables|Default|GetReverse)))))
    (Pawn|Input|AddMovementInput _output_get 1.0 false)))

(event Input|EnhancedActionEvents|EnhancedInputActionIA_Boost
  (params (ActionValue :type Boolean) (ElapsedSeconds :type Float%20%28double-precision%29) (TriggeredSeconds :type Float%20%28double-precision%29) (InputAction :type Input%20Action%20Object%20Reference :default "/Game/Input/IA_Boost.IA_Boost"))
  (:Started
    (CallFunction|BoostActive))
  (:Completed
    (CallFunction|BoostDeactive)))

(event EventBeginPlay
  ;[0.15 0.15 0.15 0.5] 기본 움직임 속도 설정
  (Variables|/Script/Engine.CharacterMovementComponent|SetMaxFlySpeed (Variables|Character|GetCharacterMovement) (Variables|Default|GetNormalSpeed)))

(event EventTick
  (params (DeltaSeconds :type Float%20%28single-precision%29))
  (if (Variables|Default|GetbIsBoosting)
    (Variables|Default|SetLeftBoostAmount (- (Variables|Default|GetLeftBoostAmount) (* DeltaSeconds (Variables|Default|GetUseBoostPerSecond))))
    (Utilities|IsBoostLeft
      (:True
        _)
      (:False
        (CallFunction|BoostDeactive)))
    (Development|PrintString (Utilities|String|ToString(Float) (Variables|Default|GetLeftBoostAmount)))))

(fn ConstructionScript)